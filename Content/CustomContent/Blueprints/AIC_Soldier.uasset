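; AI controller for soldier characters that runs the AIT_Soldier behavior tree on BeginPlay.
; When perception updates and the blackboard has no valid Enemy, it scans perceived actors and stores the first living PlayerCharacter under that key.
; An existing valid Enemy is never replaced or cleared here.
; Tick checks whether the controlled BaseCharacter is dead but takes no action.
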(event `self.ReceiveBeginPlay`
  (`self.RunBehaviorTree` "/Game/CustomContent/Blueprints/AIT_Soldier.AIT_Soldier"))

(event `self.ReceiveTick`
  (params (DeltaSeconds :type "Float (single-precision)"))
  (bind _asbase_character (cast `/Game/ThirdPersonBP/Blueprints/BaseCharacter` (`self.K2_GetPawn`)))
  (if (`/Game/ThirdPersonBP/Blueprints/BaseCharacter.IsDead` _asbase_character)
    _))

(event `self.AIPerception.OnPerceptionUpdated`
  (params (UpdatedActors :type "Array of Actor Object Reference (by ref)"))
  (bind _returnvalue (`AIBlueprintHelperLibrary.GetBlackboard` self))
  (`/Engine/EditorBlueprintResources/StandardMacros.IsValid` (`BlackboardComponent.GetValueAsObject` _returnvalue "Enemy")
    (:`Is Not Valid`
      (for _array_element (`AIPerceptionComponent.GetCurrentlyPerceivedActors` (`self.AIPerception`) null)
        (bind _asplayer_character (cast `/Game/ThirdPersonBP/Blueprints/PlayerCharacter` _array_element))
        (if (not (`/Game/ThirdPersonBP/Blueprints/BaseCharacter.IsDead` _asplayer_character))
          (`BlackboardComponent.SetValueAsObject` _returnvalue "Enemy" _asplayer_character)
          (break))))))

(fn `UserConstructionScript`)